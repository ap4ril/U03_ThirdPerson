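; Enemy AI Blueprint that sets up a great sword and a controller name label when play begins.
; After the parent BeginPlay, it writes the possessing controller's object name into the ControllerName text.
; It then attaches GreatSword to the Mesh's Hand_GreatSword socket, keeping relative transforms.
; Overlap and Tick events are empty, and the construction script only calls its parent.
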(event `self.ReceiveBeginPlay`
  (`parent.ReceiveBeginPlay`)
  (`TextRenderComponent.K2_SetText` (`self.ControllerName`) (`KismetTextLibrary.Conv_StringToText` (`KismetSystemLibrary.GetObjectName` (`self.GetController`))))
  (`self.K2_AttachToComponent` (`self.GreatSword`) (`self.Mesh`) "Hand_GreatSword" "KeepRelative" "KeepRelative" "KeepRelative" true))

(fn `UserConstructionScript`
  (`parent.UserConstructionScript`))