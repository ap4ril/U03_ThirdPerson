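; BP_Door is a sliding double door that opens automatically while the player overlaps it and closes when they leave.
; A single timeline slides the two door panels apart in opposite directions and rotates the lock, playing forward on enter and reversing on exit.
; A dynamic material on the lock switches its emissive glow to green when opening starts, then to red once closing finishes.
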(event `self.ReceiveBeginPlay`
  (bind _returnvalue (`KismetMaterialLibrary.CreateDynamicMaterialInstance` "/Game/Materials/MAT_DoorLock_Inst.MAT_DoorLock_Inst"))
  (bind _output_get (set `self.DynamicMaterial` _returnvalue))
  (`PrimitiveComponent.SetMaterial` (`self.Lock`) 0 _output_get))

(event `self.ReceiveActorBeginOverlap`
  (params (OtherActor :type "Actor Object Reference"))
  (cast `/Game/Player/BP_Player` OtherActor)
  (`MaterialInstanceDynamic.SetVectorParameterValue` (`self.DynamicMaterial`) "Emissive" (`KismetMathLibrary.MakeColor` 0.203948 20.0 0.601865))
  (bind (_direction _openlocation _lockrotation) (`Timeline|DoorTimeline` :!label _label)
    (:`Update`
      (`SceneComponent.K2_SetRelativeLocation` (`self.RightDoor`) (`KismetMathLibrary.MakeVector` 0.0 _openlocation) false false)
      (`SceneComponent.K2_SetRelativeLocation` (`self.LeftDoor`) (`KismetMathLibrary.MakeVector` 0.0 (* _openlocation -1.0)) false false)
      (`SceneComponent.K2_SetRelativeRotation` (`self.Lock`) (`KismetMathLibrary.MakeRotator` _lockrotation) false false))
    (:`Finished`
      (if (`|EnumEquality` _direction "Backward")
        (`MaterialInstanceDynamic.SetVectorParameterValue` (`self.DynamicMaterial`) "Emissive" (`KismetMathLibrary.MakeColor` 20.0 0.601865 0.203948))))))

(event `self.ReceiveActorEndOverlap`
  (params (OtherActor :type "Actor Object Reference"))
  (cast `/Game/Player/BP_Player` OtherActor)
  (goto _label :!via `Reverse`))

(fn `UserConstructionScript`)